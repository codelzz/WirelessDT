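; BP_WiTracingManager drives per-frame WiTracing renders of wireless signals from the selected receiver's transform and feeds the results to the main widget.
; Each Tick steps round-robin through BP_WirelessTransmitter actors, rendering per transmitter if one is selected, otherwise using the general render.
; Non-selected transmitters render into a temporary target, while matching or unfiltered renders use RT_WiTracing and update the RSSI PDF and player trajectory plots.
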(event EventBeginPlay
  (Utilities|FlowControl|Sequence
    (:then_0
      ;[1 1 1] Store Controller for easy access
      (bind _asbp_player_controller (Utilities|Casting|CastToBP_PlayerController (Game|GetPlayerController (Game|GetPlayerState 0))))
      (Variables|Default|SetController _asbp_player_controller))
    (:then_1
      (Rendering|ClearRenderTarget2D "/Game/WiTracing/Materials/WiTracingRenderer/RT_WiTracing.RT_WiTracing" "(R=0.208333,G=0.208333,B=0.208333,A=1.000000)"))))

(event EventTick
  (params (DeltaSeconds :type Float%20%28single-precision%29))
  (bind _controller (Variables|Default|GetController))
  (bind _mainwidget (Variables|/Game/WiTracing/Game/BP_PlayerController.BP_PlayerController_C|GetMainWidget _controller))
  (bind (_rssipdf _succeed _ismatched _nospecified) (Renderer|IterativeRenderWiTracing))
  (if (or _ismatched _nospecified)
    (Default|UpdateRSSIPdfPlot _mainwidget _rssipdf)
    (Default|UpdateTrajectoryPlot _mainwidget (Transformation|GetActorLocation (Game|Player|GetPlayerPawn 0)))))

(fn ConstructionScript)

(fn IterativeRenderWiTracing
  (bind _transform (Renderer|GetRenderTransform))
  (bind (_transmitter _succeed) (Renderer|GetIterativeTransmitter))
  (bind _controller (Variables|Default|GetController))
  (bind _mainwidget (Variables|/Game/WiTracing/Game/BP_PlayerController.BP_PlayerController_C|GetMainWidget _controller))
  (bind _selectedtransmitter (Variables|/Game/WiTracing/UI/WBP_Main.WBP_Main_C|GetSelectedTransmitter _mainwidget))
  (if _succeed
    (bind _output_get (LocalVariables|SetTransmitter _transmitter))
    ;[1 1 1] Transmitter if specified
    (if (Utilities|IsValid _selectedtransmitter)
      (if (== _selectedtransmitter _output_get)
        ;[1 1 1] Specified transmitter match
        (bind _rssipdf (Class|WiTracingRendererBlueprintLibrary|RenderWiTracingbyTransmitter _transform "/Game/WiTracing/Materials/WiTracingRenderer/RT_WiTracing.RT_WiTracing" (LocalVariables|GetTransmitter)))
        (return _rssipdf true true false)
        (else
          ;[1 1 1] Specified transmitter mismatch
          (bind _rssipdf_2 (Class|WiTracingRendererBlueprintLibrary|RenderWiTracingbyTransmitter _transform "/Game/WiTracing/Materials/WiTracingRenderer/RT_WiTracing_Tmp.RT_WiTracing_Tmp" (LocalVariables|GetTransmitter)))
          (return _rssipdf_2 true false false)))
      (else
        ;[1 1 1] No transmitter specified
        (bind _rssipdf_3 (Class|WiTracingRendererBlueprintLibrary|RenderWiTracing _transform "/Game/WiTracing/Materials/WiTracingRenderer/RT_WiTracing.RT_WiTracing"))
        (return _rssipdf_3 true false true)))
    (else
      ;[1 1 1] No transmitter
      (return 0 _succeed false false))))

(fn GetIterativeTransmitter
  (bind _outactors (Actor|GetAllActorsOfClass "/Game/WiTracing/Blueprints/BP_WirelessTransmitter.BP_WirelessTransmitter_C"))
  (bind _output_get (LocalVariables|SetNumTransmitters (Utilities|Array|Length _outactors)))
  (if (> _output_get 0)
    (bind _output_get_2 (LocalVariables|SetIterativeTransmitter (Utilities|Array|Get(acopy) _outactors (Math|Integer|%(Integer) (Variables|Renderer|GetIterativeTransmitterIndex) (LocalVariables|GetNumTransmitters)))))
    (Variables|Renderer|SetIterativeTransmitterIndex (Math|Integer|%(Integer) (+ (Variables|Renderer|GetIterativeTransmitterIndex) 1) (LocalVariables|GetNumTransmitters)))
    (return _output_get_2 true)))

(fn GetRenderTransform
  (return (Transformation|GetWorldTransform (Variables|/Game/WiTracing/Game/BP_PlayerController.BP_PlayerController_C|GetSelectedReceiver (Variables|Default|GetController)))))