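; Wireless transmitter Blueprint for WiTracing that shows its own name as a floating text label.
; On BeginPlay, InitTextRender sets the TextRender to the actor's display name and makes it visible.
; Every Tick, the label copies the first player controller's rotation and adds a 180-degree local turn, billboarding it toward the player's view.
; The graphs shown contain only label logic, with no signal or tracing behavior.
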(event EventBeginPlay
  (CallFunction|InitTextRender))

(event EventTick
  (params (DeltaSeconds :type Float%20%28single-precision%29))
  (bind _textrender (Variables|Default|GetTextRender))
  (Transformation|SetWorldRotation _textrender (.Rotation (Math|Transform|BreakTransform (Transformation|GetActorTransform (Game|GetPlayerController 0)))) false false)
  (Transformation|AddLocalRotation _textrender "0,180.000000, 0" false false))

(fn ConstructionScript)

(fn InitTextRender
  (bind _textrender (Variables|Default|GetTextRender))
  (Rendering|Components|TextRender|SetText _textrender (Utilities|Text|ToText(String) (Utilities|GetDisplayName self)))
  (Rendering|SetVisibility _textrender true false))