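; Agent that runs WiTracing wireless signal renders from the player camera and feeds the main widget's RSSI PDF and trajectory plots.
; Each tick it advances round-robin through transmitters, rendering the current one if a transmitter is selected, otherwise calling the general render.
; Non-selected transmitters render to a temporary target and skip the PDF plot.
; An optional SNR denoiser zeroes bins beyond an SNR-wide window after the first non-zero bin.
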(event EventBeginPlay
  (Utilities|FlowControl|Sequence
    (:then_0
      (CallFunction|CachePlayerController))
    (:then_1
      (Rendering|ClearRenderTarget2D "/Game/WiTracing/Materials/WiTracingRenderer/RT_WiTracing.RT_WiTracing" "(R=0.208333,G=0.208333,B=0.208333,A=1.000000)"))))

(event EventTick
  (params (DeltaSeconds :type Float%20%28single-precision%29))
  (bind _controller (Variables|Default|GetController))
  (bind _mainwidget (Variables|/Game/WiTracing/Game/BP_PlayerController.BP_PlayerController_C|GetMainWidget _controller))
  (bind (_rssipdf _succeed _ismatched _nospecified) (Renderer|IterativeRenderWiTracing))
  (if (or _ismatched _nospecified)
    ;[1 1 1] Denoise if enable
    (if (Variables|Default|GetSNRDenoiserEnable)
      ;[1 1 1] Update RSSI Pdf plot
      (Default|UpdateRSSIPdfPlot _mainwidget (CallFunction|RemoveBackgroundNoise _rssipdf))
      (else
        (Default|UpdateRSSIPdfPlot _mainwidget _rssipdf))))
  ;[1 1 1] Update trajectory plot
  (Default|UpdateTrajectoryPlot _mainwidget (Transformation|GetActorLocation (Game|Player|GetPlayerPawn 0))))

(fn ConstructionScript)

(fn IterativeRenderWiTracing
  (bind _transform (Renderer|GetRenderTransform))
  (bind (_transmitter _succeed) (Renderer|GetIterativeTransmitter))
  (bind _controller (Variables|Default|GetController))
  (bind _mainwidget (Variables|/Game/WiTracing/Game/BP_PlayerController.BP_PlayerController_C|GetMainWidget _controller))
  (bind _selectedtransmitter (Variables|/Game/WiTracing/UI/WBP_Main.WBP_Main_C|GetSelectedTransmitter _mainwidget))
  (if _succeed
    (bind _output_get (LocalVariables|SetTransmitter _transmitter))
    ;[1 1 1] Transmitter if specified
    (if (Utilities|IsValid _selectedtransmitter)
      (if (== _selectedtransmitter _output_get)
        ;[1 1 1] Specified transmitter match
        (bind _rssipdf (Class|WiTracingRendererBlueprintLibrary|RenderWiTracingbyTransmitter _transform "/Game/WiTracing/Materials/WiTracingRenderer/RT_WiTracing.RT_WiTracing" (LocalVariables|GetTransmitter)))
        (return _rssipdf true true false)
        (else
          ;[1 1 1] Specified transmitter mismatch
          (bind _rssipdf_2 (Class|WiTracingRendererBlueprintLibrary|RenderWiTracingbyTransmitter _transform "/Game/WiTracing/Materials/WiTracingRenderer/RT_WiTracing_Tmp.RT_WiTracing_Tmp" (LocalVariables|GetTransmitter)))
          (return _rssipdf_2 true false false)))
      (else
        ;[1 1 1] No transmitter specified
        (bind _rssipdf_3 (Class|WiTracingRendererBlueprintLibrary|RenderWiTracing _transform "/Game/WiTracing/Materials/WiTracingRenderer/RT_WiTracing.RT_WiTracing"))
        (return _rssipdf_3 true false true)))
    (else
      ;[1 1 1] No transmitter
      (return 0 _succeed false false))))

(fn GetIterativeTransmitter
  (bind _outactors (Actor|GetAllActorsOfClass "/Game/WiTracing/Blueprints/BP_WirelessTransmitter.BP_WirelessTransmitter_C"))
  (bind _output_get (LocalVariables|SetNumTransmitters (Utilities|Array|Length _outactors)))
  (if (> _output_get 0)
    (bind _output_get_2 (LocalVariables|SetIterativeTransmitter (Utilities|Array|Get(acopy) _outactors (Math|Integer|%(Integer) (Variables|Renderer|GetIterativeTransmitterIndex) (LocalVariables|GetNumTransmitters)))))
    (Variables|Renderer|SetIterativeTransmitterIndex (Math|Integer|%(Integer) (+ (Variables|Renderer|GetIterativeTransmitterIndex) 1) (LocalVariables|GetNumTransmitters)))
    (return _output_get_2 true)))

(fn GetRenderTransform
  (return (Transformation|GetActorTransform (Variables|/Script/Engine.PlayerController|GetPlayerCameraManager (Variables|Default|GetController)))))

(fn SwitchSNRDenoiser
  (Variables|Default|SetSNRDenoiserEnable (not (Variables|Default|GetSNRDenoiserEnable))))

(fn RemoveBackgroundNoise
  (params (RSSIPdf :type Array%20of%20Integer64s))
  (bind _denoisedrssipdf (LocalVariables|GetDenoisedRSSIPdf))
  (LocalVariables|SetRSSIPdfSize (Utilities|Array|Length RSSIPdf))
  (for (_array_element _array_index) RSSIPdf
    ;[1 1 1] Set the first index and last index if max RSSI found
    ;;[1 0 0] Haven't found the max RSSI
    (if (< (LocalVariables|GetLastIndex) 0)
      (if (!= _array_element 0)
        (LocalVariables|SetLastIndex (Math|Integer|Clamp(Integer) (+ (LocalVariables|GetSNR) _array_index) 0 (- (LocalVariables|GetRSSIPdfSize) 1))))
      (Utilities|Array|Add (LocalVariables|GetDenoisedRSSIPdf) _array_element)
      (else
        ;[0 1 0] Index within max index
        (if (<= _array_index (LocalVariables|GetLastIndex))
          (Utilities|Array|Add _denoisedrssipdf _array_element)
          (else
            (Utilities|Array|Add _denoisedrssipdf 0))))))
  (return (LocalVariables|GetDenoisedRSSIPdf)))

(fn CachePlayerController
  (bind _asbp_player_controller (Utilities|Casting|CastToBP_PlayerController (Game|GetPlayerController (Game|GetPlayerState 0))))
  (Variables|Default|SetController _asbp_player_controller))