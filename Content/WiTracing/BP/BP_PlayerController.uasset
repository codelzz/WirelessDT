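; Player controller for the WiTracing project that shows the main UI and lets the player cycle through wireless transmitters.
; On BeginPlay it caches the third-person character, then creates WBP_Main and adds it to the viewport as visible.
; Tab advances an index into all BP_WirelessTransmitter actors and passes that entry to the widget.
; Past the last transmitter, it assigns the out-of-range entry and resets the index to -1.
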(event EventBeginPlay
  (CallFunction|CacheCharacter)
  (MainWidget|InitMainWidget))

(event Input|KeyboardEvents|Tab
  (params (Key :type Key%20Structure :default "None"))
  (:Pressed
    (MainWidget|SwitchMainWidgetTransmitter)))

(fn ConstructionScript)

(fn CacheCharacter
  (bind _asbp_third_person_character (Utilities|Casting|CastToBP_ThirdPersonCharacter (Game|GetPlayerCharacter 0)))
  (Variables|Default|SetBPCharacter _asbp_third_person_character))

(fn SwitchMainWidgetTransmitter
  (bind _mainwidget (Variables|MainWidget|GetMainWidget))
  (Math|Integer|IncrementInt (Variables|Default|GetSelectedTransmitterIndex)
    (:%20%20
      (bind _outactors (Actor|GetAllActorsOfClass "/Game/WiTracing/BP/BP_WirelessTransmitter.BP_WirelessTransmitter_C"))
      (if (< (Variables|Default|GetSelectedTransmitterIndex) (Utilities|Array|Length _outactors))
        (Variables|/Game/WiTracing/UI/WBP_Main.WBP_Main_C|SetSelectedTransmitter _mainwidget (Utilities|Array|Get(acopy) _outactors (Variables|Default|GetSelectedTransmitterIndex)))
        (else
          (Variables|/Game/WiTracing/UI/WBP_Main.WBP_Main_C|SetSelectedTransmitter _mainwidget (Utilities|Array|Get(acopy) _outactors (Variables|Default|GetSelectedTransmitterIndex)))
          (Variables|Default|SetSelectedTransmitterIndex -1))))))

(fn InitMainWidget
  ;[1 1 1] Create the main widget and add it to the viewport, initially not visible
  (bind _returnvalue (UserInterface|CreateWidget "/Game/WiTracing/UI/WBP_Main.WBP_Main_C"))
  (bind _output_get (Variables|MainWidget|SetMainWidget _returnvalue))
  (UserInterface|Viewport|AddtoViewport _output_get 0)
  (Widget|SetVisibility _output_get "Visible"))