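; Manager actor that runs WiTracing each tick from the player camera and feeds the results to an RSSI PDF plot in the main widget.
; On BeginPlay it caches the BP_PlayerController and clears the RT_WiTracing render target to dark grey.
; Tick renders the scene into that target using the camera transform, then passes the returned data to the controller.
; Tracing runs in actor Tick to limit its frequency.
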(event EventBeginPlay
  (Utilities|FlowControl|Sequence
    (:then_0
      ;[1 1 1] Store Controller for easy access
      (bind _asbp_player_controller (Utilities|Casting|CastToBP_PlayerController (Game|GetPlayerController (Game|GetPlayerState 0))))
      (Variables|Default|SetController _asbp_player_controller))
    (:then_1
      (Rendering|ClearRenderTarget2D "/Game/WiTracing/Materials/RT_WiTracing.RT_WiTracing" "(R=0.208333,G=0.208333,B=0.208333,A=1.000000)"))))

(event EventTick
  (params (DeltaSeconds :type Float%20%28single-precision%29))
  ;[1 1 1] We use tick in actor to limit the wi tracing frequency
  (bind _rssipdf (Class|WiTracingRendererBlueprintLibrary|RenderScenetoTexture (Transformation|GetActorTransform (Game|GetPlayerCameraManager 0)) "/Game/WiTracing/Materials/RT_WiTracing.RT_WiTracing"))
  (Default|UpdateMainWidegtRSSIPdfPlot (Variables|Default|GetController) _rssipdf))

(fn ConstructionScript)