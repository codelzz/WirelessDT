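; Player controller for the WiTracing game, handling selection of wireless transmitters and receivers.
; On begin play it caches the test character and WiTracing manager, defaults to the badge receiver and shows the main widget.
; T steps the widget through transmitter actors, with an out-of-range read before the index resets.
; R toggles between the character's badge and mobile receivers while the manager is valid.
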(event EventBeginPlay
  (Cache|CacheCharacter)
  (Cache|CacheWiTracingManager)
  (MainWidget|InitMainWidget))

(event EventTick
  (params (DeltaSeconds :type Float%20%28single-precision%29)))

(event Input|KeyboardEvents|T
  (params (Key :type Key%20Structure :default "None"))
  (:Pressed
    (MainWidget|SwitchMainWidgetTransmitter)))

(event Input|KeyboardEvents|R
  (params (Key :type Key%20Structure :default "None"))
  (bind _testcharacter (Variables|Default|GetTestCharacter))
  (bind _receivermobile (Variables|/Game/WiTracing/Blueprints/BP_TestCharacter.BP_TestCharacter_C|GetReceiverMobile _testcharacter))
  (:Pressed
    (if (Utilities|IsValid (Variables|Default|GetWiTracingManager))
      (if (== (Variables|Default|GetSelectedReceiver) _receivermobile)
        (Variables|Default|SetSelectedReceiver (Variables|/Game/WiTracing/Blueprints/BP_TestCharacter.BP_TestCharacter_C|GetReceiverBadges (Variables|Default|GetTestCharacter)))
        (else
          (Variables|Default|SetSelectedReceiver _receivermobile))))))

(fn ConstructionScript)

(fn CacheCharacter
  (bind _asbp_test_character (Utilities|Casting|CastToBP_TestCharacter (Game|GetPlayerCharacter 0)))
  (bind _output_get (Variables|Default|SetTestCharacter _asbp_test_character))
  (Variables|Default|SetSelectedReceiver (Variables|/Game/WiTracing/Blueprints/BP_TestCharacter.BP_TestCharacter_C|GetReceiverBadges _output_get)))

(fn SwitchMainWidgetTransmitter
  (bind _mainwidget (Variables|MainWidget|GetMainWidget))
  (Math|Integer|IncrementInt (Variables|Default|GetSelectedTransmitterIndex)
    (:%20%20
      (bind _outactors (Actor|GetAllActorsOfClass "/Game/WiTracing/Blueprints/BP_WirelessTransmitter.BP_WirelessTransmitter_C"))
      (if (< (Variables|Default|GetSelectedTransmitterIndex) (Utilities|Array|Length _outactors))
        (Variables|/Game/WiTracing/UI/WBP_Main.WBP_Main_C|SetSelectedTransmitter _mainwidget (Utilities|Array|Get(acopy) _outactors (Variables|Default|GetSelectedTransmitterIndex)))
        (else
          (Variables|/Game/WiTracing/UI/WBP_Main.WBP_Main_C|SetSelectedTransmitter _mainwidget (Utilities|Array|Get(acopy) _outactors (Variables|Default|GetSelectedTransmitterIndex)))
          (Variables|Default|SetSelectedTransmitterIndex -1))))))

(fn InitMainWidget
  ;[1 1 1] Create the main widget and add it to the viewport, initially not visible
  (bind _returnvalue (UserInterface|CreateWidget "/Game/WiTracing/UI/WBP_Main.WBP_Main_C"))
  (bind _output_get (Variables|MainWidget|SetMainWidget _returnvalue))
  (UserInterface|Viewport|AddtoViewport _output_get 0)
  (Widget|SetVisibility _output_get "Visible"))

(fn CacheWiTracingManager
  (bind _returnvalue (Actor|GetActorOfClass "/Game/WiTracing/Blueprints/BP_WiTracingManager.BP_WiTracingManager_C"))
  (Variables|Default|SetWiTracingManager _returnvalue))