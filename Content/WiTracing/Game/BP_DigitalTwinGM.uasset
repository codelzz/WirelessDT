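; Game mode for the WiTracing digital twin scene, which runs simulated wireless signal tracing from the player's viewpoint.
; BeginPlay caches the WiTracing agent, digital twin and all transmitters, and shows the digital twin widget.
; Each tick aligns the pawn's child-actor receiver to camera rotation and calls MultiWiTracing against all transmitters.
; Unconnected graphs hold single-transmitter tracing and simulated-versus-real RSSI plotting, including the only branch on EnableDigitalTwin.
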(event EventBeginPlay
  (CallFunction|CacheWiTracingAgent)
  (CallFunction|CacheDigitalTwin)
  (CallFunction|InitWidget)
  (CallFunction|CacheTXs))

(event EventTick
  (params (DeltaSeconds :type Float%20%28single-precision%29))
  (bind _wirelessrx (CallFunction|CachePlayerPawnRX))
  (Class|WiTracingAgent|MultiWiTracing (Variables|Default|GetWTAgent) (Variables|Default|GetWirelessTXs) _wirelessrx))

(fn ConstructionScript)

(fn CacheWiTracingAgent
  (bind _returnvalue (Actor|GetActorOfClass "/Script/WiTracingSim.WiTracingAgent"))
  (Variables|Default|SetWTAgent _returnvalue))

(fn InitWidget
  (bind _returnvalue (UserInterface|CreateWidget "/Game/WiTracing/UI/WBP_DigitalTwin.WBP_DigitalTwin_C"))
  (bind _output_get (Variables|Default|SetWidget _returnvalue))
  (UserInterface|Viewport|AddtoViewport _output_get 0)
  (Widget|SetVisibility _output_get "Visible"))

(fn CacheDigitalTwin
  (bind _returnvalue (Actor|GetActorOfClass "/Game/WiTracing/Blueprints/BP_DigitalTwin.BP_DigitalTwin_C"))
  (Variables|Default|SetDigitalTwin _returnvalue))

(fn GetDigitalTwinTransform
  (return (Transformation|GetWorldTransform (Variables|/Game/WiTracing/Blueprints/BP_DigitalTwin.BP_DigitalTwin_C|GetWirelessReceiver (Variables|Default|GetDigitalTwin)))))

(fn GetPlayerCameraTransform
  (return (Transformation|GetActorTransform (Game|GetPlayerCameraManager 0))))

(fn GetDigitialTwinRSSI
  (return (Class|KismetMathLibrary|ToInt64(Float) (.rssi (Utilities|Struct|BreakDigitalTwinData (Variables|/Script/WiTracingSim.WiTracingDigitalTwin|GetData (Variables|Default|GetDigitalTwin)))))))

(fn SwitchEnableDigitalTwin
  (bind _output_get (Variables|Default|SetbEnableDigitalTwin (not (Variables|Default|GetbEnableDigitalTwin))))
  (return _output_get))

(fn GetCameraRotation
  (return (.Rotation (Math|Transform|BreakTransform (Transformation|GetActorTransform (Game|GetPlayerCameraManager 0))))))

(fn CachePlayerPawnRX
  (bind _asbp_digital_twin_pawn (Utilities|Casting|CastToBP_DigitalTwinPawn (Game|Player|GetPlayerPawn 0)))
  (bind _aswireless_rx (Utilities|Casting|CastToWirelessRX (Variables|/Script/Engine.ChildActorComponent|GetChildActor (Variables|/Game/WiTracing/Game/BP_DigitalTwinPawn.BP_DigitalTwinPawn_C|GetWirelessRX _asbp_digital_twin_pawn))))
  (bind _output_get (Variables|Default|SetWirelessRX _aswireless_rx))
  (Transformation|SetActorRotation _output_get (CallFunction|GetCameraRotation) true)
  (return _output_get))

(fn IterativeGetTX
  (bind _wirelesstxs (Variables|Default|GetWirelessTXs))
  (if (>= (Variables|Default|GetWirelessTXIdx) 0)
    (bind _result (Math|Integer|IncrementInt (Variables|Default|GetWirelessTXIdx))
      (:%20%20
        (Variables|Default|SetWirelessTXIdx (Math|Integer|%(Integer) _result (Utilities|Array|Length _wirelesstxs)))
        (return (Utilities|Array|Get(acopy) _wirelesstxs (Variables|Default|GetWirelessTXIdx)))))
    (else
      (return 0))))

(fn CacheTXs
  (bind _outactors (Actor|GetAllActorsOfClass "/Script/Engine.WirelessTX"))
  ;[1 1 1] If no wireless TX in the scene then set index to -1
  (if (> (Utilities|Array|Length _outactors) 0)
    (Variables|Default|SetWirelessTXs _outactors)
    (else
      (Variables|Default|SetWirelessTXIdx -1))))