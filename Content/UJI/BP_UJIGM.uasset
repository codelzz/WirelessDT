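; UJI game mode that runs wireless signal tracing between placed transmitters and the receiver on a BP_TargetAI actor.
; Each tick, the WiTracingAgent traces in-range transmitters, updating their RSSI displays and drawing rainbow-colored debug trails.
; Out-of-range transmitters get default-valued results when the timestamp changes, and all results go out over WebSocket.
; A tracing preview covers either all transmitters within a fixed radius or one, cycled by NextPreview and reset by Overview.
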(event Custom|NextPreview
  (Variables|Default|SetPreviewIdx (Class|KismetMathLibrary|ToInt64(Float) (Math|Float|%(Float) (Math|Conversions|ToFloat(Integer) (+ (Variables|Default|GetPreviewIdx) 1)) (Math|Conversions|ToFloat(Integer) (+ (Utilities|Map|Length (Variables|Default|GetWirelessTXs)) 1))))))

(event Custom|Overview
  (Variables|Default|SetPreviewIdx (Class|KismetMathLibrary|ToInt64(Integer) (Utilities|Map|Length (Variables|Default|GetWirelessTXs)))))

(event EventBeginPlay
  (CallFunction|CacheWiTracingAgent)
  (CallFunction|CacheTXs)
  (CallFunction|InitWidget)
  (CallFunction|ConfigSystem)
  (Variables|Default|SetPreviewIdx (Class|KismetMathLibrary|ToInt64(Integer) (Utilities|Map|Length (Variables|Default|GetWirelessTXs)))))

(event EventTick
  (params (DeltaSeconds :type Float%20%28single-precision%29))
  (bind _wirelesstxs (Variables|Default|GetWirelessTXs))
  (bind _previewidx (Variables|Default|GetPreviewIdx))
  (bind _wtagent (Variables|Default|GetWTAgent))
  (bind _wirelessrx (Variables|Default|GetWirelessRX))
  (bind _returnvalue (Utilities|String|ToString(Integer) _previewidx))
  (bind _returnvalue_2 (Transformation|GetActorLocation _wirelessrx))
  (bind _returnvalue_3 (Utilities|String|Append "TX" _returnvalue))
  (bind (_value _returnvalue_4) (Utilities|Map|Find _wirelesstxs _returnvalue_3))
  (Utilities|FlowControl|Sequence
    (:then_0
      (Utilities|Array|Clear (Variables|Default|GetWiTracingResults)))
    (:then_1
      (bind _wireless_rx (CallFunction|CacheAIPawnRX))
      (bind _returnvalue_5 (Class|WiTracingAgent|GetTXsinRange _wtagent (Transformation|GetActorLocation _wireless_rx) (Variables|Default|GetDetectionRange)))
      (bind _results (Class|WiTracingAgent|MultiTXWiTracing _wtagent _returnvalue_5 _wireless_rx true false false))
      (for _array_element _results
        (bind _output_get (Variables|Default|SetPrevWiTracingResult _array_element))
        (Utilities|Array|Add (Variables|Default|GetWiTracingResults) (|Copy _output_get))
        (CallFunction|UpdateTXDisplayRSSI (.txname (Utilities|Struct|BreakWiTracingResult _output_get)) (.rssi (Utilities|Struct|BreakWiTracingResult _output_get)))
        (Development|PrintString (Utilities|String|Append (.txname (Utilities|Struct|BreakWiTracingResult _output_get)) ":" (Utilities|String|ToString(Integer) (.rssi (Utilities|Struct|BreakWiTracingResult _output_get)))) true true "(R=0.000000,G=0.660000,B=1.000000,A=1.000000)" 1.0 (Utilities|String|StringToName (.txname (Utilities|Struct|BreakWiTracingResult _output_get))))
        (bind _color (CallFunction|MapRssitoRainbowColor (.rssi (Utilities|Struct|BreakWiTracingResult _output_get))))
        (Rendering|Debug|DrawDebugPoint _returnvalue_2 5.0 _color 6e+01)
        (Rendering|Debug|DrawDebugString _returnvalue_2 (Utilities|String|Append (.txname (Utilities|Struct|BreakWiTracingResult _output_get)) ":" (Utilities|String|ToString(Integer) (.rssi (Utilities|Struct|BreakWiTracingResult _output_get)))) 0 _color 6e+01))
      (if (!= (.timestamp (Utilities|Struct|BreakWiTracingResult (Variables|Default|GetPrevWiTracingResult))) (Variables|Default|GetLastWiTracingTime))
        (bind _returnvalue_6 (Class|WiTracingAgent|GetTXsOutRange _wtagent (Transformation|GetActorLocation _wireless_rx) (Variables|Default|GetDetectionRange)))
        (for _array_element_2 _returnvalue_6
          (bind _output_get_2 (Variables|Default|SetPrevWiTracingResult (Utilities|Struct|MakeWiTracingResult (Utilities|GetDisplayName _array_element_2) (.X (Class|KismetMathLibrary|BreakVector3f (Transformation|GetActorLocation _array_element_2))) (.Y (Class|KismetMathLibrary|BreakVector3f (Transformation|GetActorLocation _array_element_2))) (.Z (Class|KismetMathLibrary|BreakVector3f (Transformation|GetActorLocation _array_element_2))) (.rxname (Utilities|Struct|BreakWiTracingResult (Variables|Default|GetPrevWiTracingResult))) (.rxx (Utilities|Struct|BreakWiTracingResult (Variables|Default|GetPrevWiTracingResult))) (.rxy (Utilities|Struct|BreakWiTracingResult (Variables|Default|GetPrevWiTracingResult))) (.rxz (Utilities|Struct|BreakWiTracingResult (Variables|Default|GetPrevWiTracingResult))) -255 (.timestamp (Utilities|Struct|BreakWiTracingResult (Variables|Default|GetPrevWiTracingResult))))))
          (Utilities|Array|Add (Variables|Default|GetWiTracingResults) (|Copy _output_get_2))
          (Variables|Default|SetLastWiTracingTime (.timestamp (Utilities|Struct|BreakWiTracingResult _output_get_2)))
          (CallFunction|UpdateTXDisplayRSSI (.txname (Utilities|Struct|BreakWiTracingResult _output_get_2)) (.rssi (Utilities|Struct|BreakWiTracingResult _output_get_2))))))
    (:then_2
      (if (== (Variables|Default|GetPreviewIdx) (Utilities|Map|Length (Variables|Default|GetWirelessTXs)))
        (bind _wireless_rx_2 (CallFunction|CacheAIPawnRX))
        (bind _returnvalue_7 (Class|WiTracingAgent|GetTXsinRange _wtagent (Transformation|GetActorLocation _wireless_rx_2) 1e+04))
        (Class|WiTracingAgent|PreviewWiTracing _wtagent _returnvalue_7 _wireless_rx_2 true false)
        (else
          (bind _wireless_rx_3 (CallFunction|CacheAIPawnRX))
          (if _returnvalue_4
            (Class|WiTracingAgent|PreviewWiTracing (Variables|Default|GetWTAgent) (Utilities|Array|MakeArray _value) _wireless_rx_3 true false)))))
    (:then_3
      (Class|WiTracingAgent|WebSocketSend (Variables|Default|GetWTAgent) (Variables|Default|GetWiTracingResults)))))

(fn ConstructionScript)

(fn CacheWiTracingAgent
  (bind _returnvalue (Actor|GetActorOfClass "/Script/WiTracingSim.WiTracingAgent"))
  (Variables|Default|SetWTAgent _returnvalue))

(fn InitWidget
  (bind _returnvalue (UserInterface|CreateWidget "/Game/Demo/UI/WBP_Demo.WBP_Demo_C"))
  (bind _output_get (Variables|Default|SetWidget _returnvalue))
  (UserInterface|Viewport|AddtoViewport _output_get 0)
  (Widget|SetVisibility _output_get "Visible"))

(fn GetPlayerCameraTransform
  (return (Transformation|GetActorTransform (Game|GetPlayerCameraManager 0))))

(fn GetDigitialTwinRSSI)

(fn SwitchEnableDigitalTwin
  (bind _output_get (Variables|Default|SetbEnableDigitalTwin (not (Variables|Default|GetbEnableDigitalTwin))))
  (return _output_get))

(fn GetCameraRotation
  (return (.Rotation (Math|Transform|BreakTransform (Transformation|GetActorTransform (Game|GetPlayerCameraManager 0))))))

(fn CachePlayerPawnRX
  (bind _asbp_demo_pawn (Utilities|Casting|CastToBP_DemoPawn (Game|Player|GetPlayerPawn 0)))
  (bind _aswireless_rx (Utilities|Casting|CastToWirelessRX (Variables|/Script/Engine.ChildActorComponent|GetChildActor (Variables|/Game/Demo/Game/BP_DemoPawn.BP_DemoPawn_C|GetWirelessRX _asbp_demo_pawn))))
  (bind _output_get (Variables|Default|SetWirelessRX _aswireless_rx))
  (Transformation|SetActorRotation _output_get (CallFunction|GetCameraRotation) true)
  (return _output_get))

(fn CacheAIPawnRX
  (bind _returnvalue (Actor|GetActorOfClass "/Game/Demo/Character/BP_TargetAI.BP_TargetAI_C"))
  (bind _aswireless_rx (Utilities|Casting|CastToWirelessRX (Variables|/Script/Engine.ChildActorComponent|GetChildActor (Variables|/Game/Demo/Character/BP_TargetAI.BP_TargetAI_C|GetRX _returnvalue))))
  (bind _output_get (Variables|Default|SetWirelessRX _aswireless_rx))
  (return _output_get))

(fn CacheTXs
  (bind _outactors (Actor|GetAllActorsOfClass "/Game/Demo/Device/BP_WirelessTX.BP_WirelessTX_C"))
  (for _array_element _outactors
    (Utilities|Map|Add (Variables|Default|GetWirelessTXs) (Utilities|GetDisplayName _array_element) _array_element)))

(fn ConfigSystem
  (Development|ExecuteConsoleCommand (Utilities|String|Append "ShowFlag.Splines" " " "1") 0))

(fn UpdateTXDisplayRSSI
  (params (TXName :type String) (RSSI :type Integer64))
  (bind _wirelesstxs (Variables|Default|GetWirelessTXs))
  (bind (_value _returnvalue) (Utilities|Map|Find _wirelesstxs TXName))
  (if _returnvalue
    (Default|UpdateDisplayRSSI _value RSSI)))