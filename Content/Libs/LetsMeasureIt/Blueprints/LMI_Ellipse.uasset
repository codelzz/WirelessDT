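; LMI_Ellipse is a Let's Measure It actor that displays an ellipse's area, dimensions and approximate circumference as text.
; LMIUpdate, also run from the construction script, derives the figures from actor X/Y scale in meters, locking Z to 1.
; A valid Control can override the cylinder's material through GetControlValues, extending the parent's version.
; The label gets scale-corrected transform, color and camera-facing setup, and can stay centered on the actor.
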(event EventLMIUpdate
  (bind _returnvalue (Transformation|GetActorScale3D))
  (bind _returnvalue_2 (Transformation|GetActorScale3D))
  (bind _returnvalue_3 (Transformation|GetActorScale3D))
  (bind _returnvalue_4 (Transformation|GetActorScale3D))
  (bind (_x _y) (Math|Vector|BreakVector _returnvalue_3))
  (bind (_x_2 _y_2) (Math|Vector|BreakVector _returnvalue_4))
  (CallFunction|GetControlValues)
  ;[1 1 1] Ignore the Z axis scaling
  (Transformation|SetActorScale3D (Math|Vector|MakeVector (.x _returnvalue) (.y _returnvalue) 1.0))
  ;[1 1 1] Get the circumference
  (bind _circumference (CallFunction|CalcOvalCircumference (/ _x 2.0) (/ _y 2.0)))
  ;[1 1 1] Build text string
  (Rendering|Components|TextRender|SetText (Variables|Default|GetTextRender) (Utilities|Text|FormatText "{name}<br>Area: {Area}m2 ({Width}m x {Height}m)<br>Circumference: ~{Circumference}m" (Utilities|Text|ToText(String) (Utilities|GetDisplayName self)) (Utilities|Text|ToText(Float) (Math|Float|MultiplybyPi (* (/ _x_2 2.0) (/ _y_2 2.0))) "HalfToEven" false true 1 324 0 2) (Utilities|Text|ToText(Float) (.x _returnvalue_2) "HalfToEven" false true 1 324 0 2) (Utilities|Text|ToText(Float) (.y _returnvalue_2) "HalfToEven" false true 1 324 0 2) (Utilities|Text|ToText(Float) _circumference "HalfToEven" false true 1 324 0 2)))
  ;[1 1 1] Set the textrender color, transform
  (CallFunction|SetupTextTransform (Variables|Default|GetTextRender) (Variables|Default|GetTextColor) self (CallFunction|CorrectActorScale (Variables|Default|GetControl) (Variables|Default|GetTextTransform) self) (Variables|Default|GetFaceCamera))
  ;[1 1 1] Material
  (Rendering|Material|SetMaterial (Variables|Default|GetCylinder) 0 (Variables|Default|GetMaterial))
  (CallFunction|SetKeepTextCentered))

(event EventGetControlValues
  (bind _control (Variables|Default|GetControl))
  (bind _ellipsematerial (Variables|/Game/Libs/LetsMeasureIt/Blueprints/LMI_Control.LMI_Control_C|GetEllipseMaterial _control))
  (|CallParentFunction)
  (Utilities|IsValid (Variables|Default|GetControl)
    (:Is%20Valid
      (Utilities|IsValid _ellipsematerial
        (:Is%20Valid
          (Variables|Default|SetMaterial _ellipsematerial))))))

(fn ConstructionScript
  (CallFunction|LMIUpdate))

(fn SetKeepTextCentered
  (bind _returnvalue (Transformation|GetActorLocation))
  (bind (_x _y _z) (Math|Vector|BreakVector _returnvalue))
  (if (Variables|Default|GetKeepTextCentered)
    (Transformation|SetWorldLocation (Variables|Default|GetTextRender) (Math|Vector|MakeVector _x _y (+ _z (.z (.Location (Math|Transform|BreakTransform (Variables|Default|GetTextTransform)))))) false false)))