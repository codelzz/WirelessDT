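; LetsMeasureIt rectangle actor that turns its X/Y scale into meters and displays name, area, size and circumference as text.
; LMIUpdate, run from the construction script, offsets the plane so the pivot sits at a corner and locks Z scale to 1.
; It extends parent control values with the Control's rectangle material, then applies material and text transform, optionally centering the text over the plane.
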(event EventLMIUpdate
  (bind _returnvalue (Transformation|GetActorScale3D))
  (bind _returnvalue_2 (Transformation|GetActorScale3D))
  (bind _returnvalue_3 (Transformation|GetActorScale3D))
  (bind _returnvalue_4 (Transformation|GetActorScale3D))
  (bind _returnvalue_5 (Transformation|GetActorScale3D))
  (bind _returnvalue_6 (* _returnvalue_5 1e+02))
  (bind _returnvalue_7 (/ _returnvalue_6 2.0))
  (bind (_x _y) (Math|Vector|BreakVector _returnvalue_7))
  (CallFunction|GetControlValues)
  ;[1 1 1] Set the plan corners to the pivot
  (Transformation|SetWorldLocation (Variables|Default|GetPlane) (+ (Math|Vector|MakeVector _x _y 0.0) (Transformation|GetActorLocation)) false false)
  ;[1 1 1] Ignore the Z axis scaling
  (Transformation|SetActorScale3D (Math|Vector|MakeVector (.x _returnvalue) (.y _returnvalue) 1.0))
  ;[1 1 1] Calculate the Area
  (Variables|Default|SetArea (* (.x _returnvalue_3) (.y _returnvalue_3)))
  ;[1 1 1] Calculate the Circumference
  (bind _circumference (CallFunction|CalcRectangleCircumference (.x _returnvalue_2) (.y _returnvalue_2)))
  ;[1 1 1] Build text
  (Rendering|Components|TextRender|SetText (Variables|Default|GetTextRender) (Utilities|Text|FormatText "{name}<br>Area: {Area}m2 ({Width}m x {Height}m)<br>Circumference: {Circumference}m" (Utilities|Text|ToText(String) (Utilities|GetDisplayName self)) (Utilities|Text|ToText(Float) (Variables|Default|GetArea) "HalfToEven" false true 1 324 0 2) (Utilities|Text|ToText(Float) (.x _returnvalue_4) "HalfToEven" false true 1 324 0 2) (Utilities|Text|ToText(Float) (.y _returnvalue_4) "HalfToEven" false true 1 324 0 2) (Utilities|Text|ToText(Float) _circumference "HalfToEven" false true 1 324 0 2)))
  ;[1 1 1] Set the textrender color, transform
  (CallFunction|SetupTextTransform (Variables|Default|GetTextRender) (Variables|Default|GetTextColor) self (CallFunction|CorrectActorScale (Variables|Default|GetControl) (Variables|Default|GetTextTransform) self) (Variables|Default|GetFaceCamera))
  ;[1 1 1] Set Material
  (Rendering|Material|SetMaterial (Variables|Default|GetPlane) 0 (Variables|Default|GetMaterial))
  (CallFunction|SetKeepTextCentered))

(event EventGetControlValues
  (bind _control (Variables|Default|GetControl))
  (bind _rectanglematerial (Variables|/Game/LetsMeasureIt/Blueprints/LMI_Control.LMI_Control_C|GetRectangleMaterial _control))
  (|CallParentFunction)
  (Utilities|IsValid (Variables|Default|GetControl)
    (:Is%20Valid
      ;[1 1 1] Get the material from the LMI Control
      (Utilities|IsValid _rectanglematerial
        (:Is%20Valid
          (Variables|Default|SetMaterial _rectanglematerial))))))

(fn ConstructionScript
  (CallFunction|LMIUpdate))

(fn SetKeepTextCentered
  (bind _returnvalue (Transformation|GetActorScale3D))
  (bind _returnvalue_2 (Transformation|GetActorLocation))
  (bind _returnvalue_3 (* _returnvalue 1e+02))
  (bind _returnvalue_4 (/ _returnvalue_3 2.0))
  (bind (_x _y) (Math|Vector|BreakVector _returnvalue_4))
  (bind _returnvalue_5 (Math|Vector|MakeVector _x _y 0.0))
  (bind _returnvalue_6 (+ _returnvalue_5 _returnvalue_2))
  (bind (_x_2 _y_2 _z) (Math|Vector|BreakVector _returnvalue_6))
  (if (Variables|Default|GetKeepTextCentered)
    (Transformation|SetWorldLocation (Variables|Default|GetTextRender) (Math|Vector|MakeVector _x_2 _y_2 (+ _z (.z (.location (Variables|Default|GetTextTransform))))) false false)))