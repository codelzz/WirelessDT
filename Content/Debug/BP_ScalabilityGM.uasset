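; Debug game mode, apparently for scalability testing of multi-transmitter WiTracing, the wireless signal tracing between TX and RX actors.
; BeginPlay caches the tracing agent, all WirelessTX actors and a training agent, adds a debug widget and shows splines.
; Each tick aligns the debug pawn's receiver to the camera, traces every transmitter in one call with optional octahedral projection, and prints result count and FPS.
; Per-transmitter RSSI reporting is disconnected.
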(event EventBeginPlay
  (CallFunction|CacheWiTracingAgent)
  (CallFunction|CacheTXs)
  (CallFunction|InitWidget)
  (CallFunction|ConfigSystem)
  (bind _returnvalue (Actor|GetActorOfClass "/Script/WiTracingSim.TrainingAgent"))
  (Variables|Default|SetTrainingAgent _returnvalue)
  (Variables|Default|SetPreviousFrameTime (Utilities|Time|GetGameTimeinSeconds)))

(event EventTick
  (params (DeltaSeconds :type Float%20%28single-precision%29))
  (Utilities|FlowControl|Sequence
    (:then_0
      (bind _wirelessrx (CallFunction|CachePlayerPawnRX))
      (bind _results (Class|WiTracingAgent|MultiTXWiTracing (Variables|Default|GetWTAgent) (Variables|Default|GetWirelessTXs) _wirelessrx (Variables|Default|GetEnableOctahedralProjection) false false))
      (Development|PrintString (Utilities|String|ToString(Integer) (Utilities|Array|Length _results)) true true "(R=0.000000,G=0.660000,B=1.000000,A=1.000000)" 2.0 "1"))
    (:then_1
      (Development|PrintString (Utilities|String|ToString(Float) (/ 1.0 DeltaSeconds)) true false "(R=0.000000,G=0.660000,B=1.000000,A=1.000000)" 2.0 "2"))))

(fn ConstructionScript)

(fn CacheWiTracingAgent
  (bind _returnvalue (Actor|GetActorOfClass "/Script/WiTracingSim.WiTracingAgent"))
  (Variables|Default|SetWTAgent _returnvalue))

(fn InitWidget
  (bind _returnvalue (UserInterface|CreateWidget "/Game/Debug/WBP_WiTracing_DBG.WBP_WiTracing_DBG_C"))
  (bind _output_get (Variables|Default|SetWidget _returnvalue))
  (UserInterface|Viewport|AddtoViewport _output_get 0)
  (Widget|SetVisibility _output_get "Visible"))

(fn GetPlayerCameraTransform
  (return (Transformation|GetActorTransform (Game|GetPlayerCameraManager 0))))

(fn GetDigitialTwinRSSI)

(fn SwitchEnableDigitalTwin)

(fn GetCameraRotation
  (return (.Rotation (Math|Transform|BreakTransform (Transformation|GetActorTransform (Game|GetPlayerCameraManager 0))))))

(fn CachePlayerPawnRX
  (bind _asbp_debug_pawn (Utilities|Casting|CastToBP_DebugPawn (Game|Player|GetPlayerPawn 0)))
  (bind _aswireless_rx (Utilities|Casting|CastToWirelessRX (Variables|/Script/Engine.ChildActorComponent|GetChildActor (Variables|/Game/Debug/BP_DebugPawn.BP_DebugPawn_C|GetWirelessRX _asbp_debug_pawn))))
  (bind _output_get (Variables|Default|SetWirelessRX _aswireless_rx))
  (Transformation|SetActorRotation _output_get (CallFunction|GetCameraRotation) true)
  (return _output_get))

(fn CacheAIPawnRX
  (bind _returnvalue (Actor|GetActorOfClass "/Game/Demo/Character/BP_TargetAI.BP_TargetAI_C"))
  (bind _aswireless_rx (Utilities|Casting|CastToWirelessRX (Variables|/Script/Engine.ChildActorComponent|GetChildActor (Variables|/Game/Demo/Character/BP_TargetAI.BP_TargetAI_C|GetRX _returnvalue))))
  (bind _output_get (Variables|Default|SetWirelessRX _aswireless_rx))
  (return _output_get))

(fn CacheTXs
  (bind _outactors (Actor|GetAllActorsOfClass "/Script/Engine.WirelessTX"))
  (Variables|Default|SetWirelessTXs _outactors))

(fn ConfigSystem
  (Development|ExecuteConsoleCommand (Utilities|String|Append "ShowFlag.Splines" " " "1") 0))