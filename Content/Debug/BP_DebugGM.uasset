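; Debug game mode that runs live WiTracing wireless signal simulation from the player pawn and shows per-transmitter RSSI.
; BeginPlay caches the tracing agent and transmitters, adds a debug widget and enables spline display.
; Each tick it aligns the pawn's receiver to camera rotation, previews and traces transmitters in range, then updates their RSSI displays and prints values.
; Results are then sent over the agent's WebSocket.
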(event EventBeginPlay
  (CallFunction|CacheWiTracingAgent)
  (CallFunction|CacheTXs)
  (CallFunction|InitWidget)
  (CallFunction|ConfigSystem)
  (bind _returnvalue (Actor|GetActorOfClass "/Script/WiTracingSim.TrainingAgent"))
  (Variables|Default|SetTrainingAgent _returnvalue))

(event EventTick
  (params (DeltaSeconds :type Float%20%28single-precision%29))
  (Utilities|FlowControl|Sequence
    (:then_0
      (Utilities|Array|Clear (Variables|Default|GetWiTracingResults)))
    (:then_1
      (bind _wirelessrx (CallFunction|CachePlayerPawnRX))
      (bind _returnvalue (Class|WiTracingAgent|GetTXsinRange (Variables|Default|GetWTAgent) (Transformation|GetActorLocation _wirelessrx) 1e+04))
      (Class|WiTracingAgent|PreviewWiTracing (Variables|Default|GetWTAgent) _returnvalue _wirelessrx (Variables|Default|GetEnableOctahedralProjection) false)
      (bind _results (Class|WiTracingAgent|MultiTXWiTracing (Variables|Default|GetWTAgent) _returnvalue _wirelessrx true false false))
      (for _array_element _results
        (Utilities|Array|Add (Variables|Default|GetWiTracingResults) (|Copy _array_element))
        (CallFunction|UpdateTXDisplayRSSI (.txname (Utilities|Struct|BreakWiTracingResult (|Copy _array_element))) (.rssi (Utilities|Struct|BreakWiTracingResult (|Copy _array_element))))
        (Development|PrintString (Utilities|String|Append (.txname (Utilities|Struct|BreakWiTracingResult (|Copy _array_element))) ":" (Utilities|String|ToString(Integer) (.rssi (Utilities|Struct|BreakWiTracingResult (|Copy _array_element))))) true true "(R=0.000000,G=0.660000,B=1.000000,A=1.000000)" 1.0 (Utilities|String|StringToName (.txname (Utilities|Struct|BreakWiTracingResult (|Copy _array_element)))))))
    (:then_2
      (Class|WiTracingAgent|WebSocketSend (Variables|Default|GetWTAgent) (Variables|Default|GetWiTracingResults)))))

(fn ConstructionScript)

(fn CacheWiTracingAgent
  (bind _returnvalue (Actor|GetActorOfClass "/Script/WiTracingSim.WiTracingAgent"))
  (Variables|Default|SetWTAgent _returnvalue))

(fn InitWidget
  (bind _returnvalue (UserInterface|CreateWidget "/Game/Debug/WBP_WiTracing_DBG.WBP_WiTracing_DBG_C"))
  (bind _output_get (Variables|Default|SetWidget _returnvalue))
  (UserInterface|Viewport|AddtoViewport _output_get 0)
  (Widget|SetVisibility _output_get "Visible"))

(fn GetPlayerCameraTransform
  (return (Transformation|GetActorTransform (Game|GetPlayerCameraManager 0))))

(fn GetDigitialTwinRSSI)

(fn SwitchEnableDigitalTwin)

(fn GetCameraRotation
  (return (.Rotation (Math|Transform|BreakTransform (Transformation|GetActorTransform (Game|GetPlayerCameraManager 0))))))

(fn CachePlayerPawnRX
  (bind _asbp_debug_pawn (Utilities|Casting|CastToBP_DebugPawn (Game|Player|GetPlayerPawn 0)))
  (bind _aswireless_rx (Utilities|Casting|CastToWirelessRX (Variables|/Script/Engine.ChildActorComponent|GetChildActor (Variables|/Game/Debug/BP_DebugPawn.BP_DebugPawn_C|GetWirelessRX _asbp_debug_pawn))))
  (bind _output_get (Variables|Default|SetWirelessRX _aswireless_rx))
  (Transformation|SetActorRotation _output_get (CallFunction|GetCameraRotation) true)
  (return _output_get))

(fn CacheAIPawnRX
  (bind _returnvalue (Actor|GetActorOfClass "/Game/Demo/Character/BP_TargetAI.BP_TargetAI_C"))
  (bind _aswireless_rx (Utilities|Casting|CastToWirelessRX (Variables|/Script/Engine.ChildActorComponent|GetChildActor (Variables|/Game/Demo/Character/BP_TargetAI.BP_TargetAI_C|GetRX _returnvalue))))
  (bind _output_get (Variables|Default|SetWirelessRX _aswireless_rx))
  (return _output_get))

(fn CacheTXs
  (bind _outactors (Actor|GetAllActorsOfClass "/Game/Demo/Device/BP_WirelessTX.BP_WirelessTX_C"))
  (for _array_element _outactors
    (Utilities|Map|Add (Variables|Default|GetWirelessTXs) (Utilities|GetDisplayName _array_element) _array_element)))

(fn ConfigSystem
  (Development|ExecuteConsoleCommand (Utilities|String|Append "ShowFlag.Splines" " " "1") 0))

(fn UpdateTXDisplayRSSI
  (params (TXName :type String) (RSSI :type Integer64))
  (bind _wirelesstxs (Variables|Default|GetWirelessTXs))
  (bind (_value _returnvalue) (Utilities|Map|Find _wirelesstxs TXName))
  (if _returnvalue
    (Default|UpdateDisplayRSSI _value RSSI)))