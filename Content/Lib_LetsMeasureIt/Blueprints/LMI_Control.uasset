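; LMI_Control is a shared control actor for the LetsMeasureIt (LMI) library that propagates its property edits to the measuring actors linked to it.
; Its construction script resets the Update flag and shows the actor's display name on a TextRender.
; It then scans all LMI_Base actors and calls LMIUpdate on those whose Control references this instance.
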(fn ConstructionScript
  (Variables|Default|SetUpdate false)
  ;[1 1 1] Show the name of this component
  (Rendering|Components|TextRender|SetText (Variables|Default|GetTextRender) (Utilities|Text|ToText(String) (Utilities|GetDisplayName self)))
  ;[1 1 1] Some property on ourself has changed. Notify all LMI components to update their properties
  (bind _outactors (Actor|GetAllActorsOfClass "/Game/Lib_LetsMeasureIt/HelperBlueprints/LMI_Base.LMI_Base_C"))
  (for _array_element _outactors
    (if (== (Variables|/Game/Lib_LetsMeasureIt/HelperBlueprints/LMI_Base.LMI_Base_C|GetControl _array_element) self)
      (Default|LMIUpdate _array_element))))