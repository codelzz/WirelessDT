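; LMI_Route is a spline-based measuring actor that shows distance and estimated travel time along a route.
; The construction script places instanced point meshes at a fixed spacing, plus marker meshes and text renderers at percentage positions along the spline.
; Each label shows name, percentage, meters and seconds at the character speed.
; LMIUpdate pulls shared settings from a Control object when valid, then refreshes labels, meshes, materials and scales.
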(event EventLMIUpdate
  (CallFunction|GetControlValues)
  (CallFunction|SetupTextItems)
  ;[1 1 1] Set Point mesh and material
  (Components|StaticMesh|SetStaticMesh (Variables|Default|GetHierarchicalInstancedStaticMesh) (Variables|Points|GetPointMesh))
  (Rendering|Material|SetMaterial (Variables|Default|GetHierarchicalInstancedStaticMesh) 0 (Variables|Points|GetPointMaterial))
  ;[1 1 1] Set Point properties
  (for _index (range 0 (Components|InstancedStaticMesh|GetInstanceCount (Variables|Default|GetHierarchicalInstancedStaticMesh)))
    (Components|InstancedStaticMesh|UpdateInstanceTransform (Variables|Default|GetHierarchicalInstancedStaticMesh) _index (Math|Transform|MakeTransform (.location (.OutInstanceTransform (Components|InstancedStaticMesh|GetInstanceTransform (Variables|Default|GetHierarchicalInstancedStaticMesh) _index false))) (.rotation (.OutInstanceTransform (Components|InstancedStaticMesh|GetInstanceTransform (Variables|Default|GetHierarchicalInstancedStaticMesh) _index false))) (Math|Conversions|ToVector(Float) (Variables|Points|GetPointScale))) false true false))
  ;[1 1 1] Set Marker properties
  (for _array_element (Variables|Default|GetMarkers)
    (Components|StaticMesh|SetStaticMesh _array_element (Variables|Markers|GetMarkerMesh))
    (Rendering|Material|SetMaterial _array_element 0 (Variables|Markers|GetMarkerMaterial))
    (Transformation|SetWorldScale3D _array_element (Math|Conversions|ToVector(Float) (Variables|Markers|GetMarkerScale)))))

(event EventGetControlValues
  (|CallParentFunction)
  (Utilities|IsValid (Variables|Default|GetControl)
    (:Is%20Valid
      (Variables|Points|SetPointMesh (Variables|/Game/Lib_LetsMeasureIt/Blueprints/LMI_Control.LMI_Control_C|GetPoint%20Mesh (Variables|Default|GetControl)))
      (Variables|Points|SetPointMaterial (Variables|/Game/Lib_LetsMeasureIt/Blueprints/LMI_Control.LMI_Control_C|GetPoint%20Material (Variables|Default|GetControl)))
      (Variables|Markers|SetMarkerMesh (Variables|/Game/Lib_LetsMeasureIt/Blueprints/LMI_Control.LMI_Control_C|GetMarker%20Mesh (Variables|Default|GetControl)))
      (Variables|Markers|SetMarkerMaterial (Variables|/Game/Lib_LetsMeasureIt/Blueprints/LMI_Control.LMI_Control_C|GetMarker%20Material (Variables|Default|GetControl)))
      (Variables|Default|SetCharacterSpeed (Variables|/Game/Lib_LetsMeasureIt/Blueprints/LMI_Control.LMI_Control_C|GetCharacterSpeed (Variables|Default|GetControl)))
      (Variables|Markers|SetMarkerScale (Variables|/Game/Lib_LetsMeasureIt/Blueprints/LMI_Control.LMI_Control_C|GetMarkerScale (Variables|Default|GetControl)))
      (Variables|Points|SetPointScale (Variables|/Game/Lib_LetsMeasureIt/Blueprints/LMI_Control.LMI_Control_C|GetPointScale (Variables|Default|GetControl))))))

(fn ConstructionScript
  ;[1 1 1] Setup Hierarchical Instanced Mesh( no shadow, the static Mesh to use and Material )
  (Rendering|SetCastShadow (Variables|Default|GetHierarchicalInstancedStaticMesh) false)
  (Components|StaticMesh|SetStaticMesh (Variables|Default|GetHierarchicalInstancedStaticMesh) (Variables|Points|GetPointMesh))
  (Rendering|Material|SetMaterial (Variables|Default|GetHierarchicalInstancedStaticMesh) 0 (Variables|Points|GetPointMaterial))
  (for _index (range 1 (Math|Float|Truncate (/ (Spline|GetSplineLength (Variables|Default|GetSpline)) (* (Variables|Points|GetPointDistance) 1e+02))))
    ;[1 1 1] FOREACH add a point mesh along the spline
    (Class|InstancedStaticMeshComponent|AddInstanceWorldSpace (Variables|Default|GetHierarchicalInstancedStaticMesh) (Math|Transform|MakeTransform (Spline|GetLocationatDistanceAlongSpline (Variables|Default|GetSpline) (* _index (* (Variables|Points|GetPointDistance) 1e+02)) "World") "0, 0, 0" (Math|Conversions|ToVector(Float) (Variables|Points|GetPointScale)))))
  ;[1 1 1] Call SetupText to add Text
  (CallFunction|SetupTextComponents)
  (Utilities|Array|Clear (Variables|Default|GetMarkers))
  ;[1 1 1] Add Markers
  (for _array_element (Variables|Markers|GetDistanceMarkers)
    (bind _returnvalue (AddComponent|AddStaticMeshComponent false (Math|Conversions|ToTransform(Vector) (Spline|GetLocationatDistanceAlongSpline (Variables|Default|GetSpline) (* _array_element (/ (Spline|GetSplineLength (Variables|Default|GetSpline)) 1e+02)) "Local"))))
    (Utilities|Array|Add (Variables|Default|GetMarkers) _returnvalue)
    (Components|StaticMesh|SetStaticMesh _returnvalue (Variables|Markers|GetMarkerMesh))
    (Rendering|Material|SetMaterial _returnvalue 0 (Variables|Markers|GetMarkerMaterial))
    (Transformation|SetWorldScale3D _returnvalue (Math|Conversions|ToVector(Float) (Variables|Markers|GetMarkerScale)))
    (Collision|SetCollisionEnabled _returnvalue "NoCollision")
    (Rendering|SetCastShadow _returnvalue false))
  (CallFunction|LMIUpdate))

(fn SetupTextComponents
  ;[1 1 1] FOREACH Distance Marker
  (Utilities|Array|Clear (Variables|Default|GetTextRenderers))
  (for _array_element (Variables|Markers|GetDistanceMarkers)
    ;[1 1 1] Setup Text component
    (bind _returnvalue (AddComponent|AddTextRenderComponent false))
    (bind _output_get (LocalVariables|SetCurrentTextRender _returnvalue))
    (Utilities|Array|Add (Variables|Default|GetTextRenderers) _output_get)
    ;[1 1 1] Set text Horizontal Alignment
    (Rendering|Components|TextRender|SetHorizontalAlignment (LocalVariables|GetCurrentTextRender) "EHTA_Center"))
  (CallFunction|SetupTextItems))

(fn SetupTextItems
  (bind _texttransform (Variables|Default|GetTextTransform))
  (bind _texttransform_2 (Variables|Default|GetTextTransform))
  (Transformation|SetActorScale3D "1.000000,1.000000,1.000000") ; Prevent scaling of the actor itself
  (for (_array_element _array_index) (Variables|Default|GetTextRenderers)
    ;[1 1 1] Create the text and set TextRender
    (bind _text (CallFunction|CreateTextString (Utilities|Array|Get(acopy) (Variables|Markers|GetDistanceMarkers) _array_index)))
    (Rendering|Components|TextRender|SetText _array_element _text)
    ;[1 1 1] IF KeepTextCentered
    (if (Variables|Default|GetKeepTextCentered)
      ;[1 1 1] We need to keep the text centered over the distance markers
      (LocalVariables|SetFinalTextTransform (Math|Transform|MakeTransform (Math|Vector|MakeVector (.X (Math|Vector|BreakVector (CallFunction|GetLocationatSpline (Utilities|Array|Get(acopy) (Variables|Markers|GetDistanceMarkers) _array_index)))) (.Y (Math|Vector|BreakVector (CallFunction|GetLocationatSpline (Utilities|Array|Get(acopy) (Variables|Markers|GetDistanceMarkers) _array_index)))) (+ (.Z (Math|Vector|BreakVector (CallFunction|GetLocationatSpline (Utilities|Array|Get(acopy) (Variables|Markers|GetDistanceMarkers) _array_index)))) (.Z (Math|Vector|BreakVector (.location _texttransform))))) (.rotation _texttransform) (.scale _texttransform)))
      (else
        ;[1 1 1] The text should be placed based on Text Transform, relative to the distance markers
        (LocalVariables|SetFinalTextTransform (Math|Transform|MakeTransform (+ (CallFunction|GetLocationatSpline (Utilities|Array|Get(acopy) (Variables|Markers|GetDistanceMarkers) _array_index)) (.location _texttransform_2)) (.rotation _texttransform_2) (.scale _texttransform_2)))))
    (CallFunction|SetupTextTransform _array_element (Variables|Default|GetTextColor) self (LocalVariables|GetFinalTextTransform) (Variables|Default|GetFaceCamera))))

(fn CreateTextString
  (params (DistanceMarkerValue :type Float%20%28double-precision%29))
  (bind _spline (Variables|Default|GetSpline))
  (bind _returnvalue (Spline|GetSplineLength _spline))
  (return (Utilities|Text|FormatText "{Name}({DistancePercentage}%)<br>{DistanceMeters}m / ~{TimeToTravel}s" (Utilities|Text|ToText(String) (Utilities|GetDisplayName self)) (Utilities|Text|ToText(Float) DistanceMarkerValue "HalfToEven" false true 1 324 0 2) (Utilities|Text|ToText(Float) (* DistanceMarkerValue (/ _returnvalue 1e+04)) "HalfToEven" false true 1 324 2 2) (Utilities|Text|ToText(Float) (/ (* _returnvalue (/ DistanceMarkerValue 1e+02)) (Variables|Default|GetCharacterSpeed)) "HalfToEven" false true 1 324 2 2))))

(fn GetLocationatSpline
  (params (DistanceAtSplinePercentage :type Float%20%28double-precision%29))
  (return (Spline|GetLocationatDistanceAlongSpline (Variables|Default|GetSpline) (* DistanceAtSplinePercentage (/ (Spline|GetSplineLength (Variables|Default|GetSpline)) 1e+02)) "Local")))