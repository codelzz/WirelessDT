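; LMI_Ruler is a measuring actor that draws a ruler between two points or linked actors, labelled with its name and length in meters.
; The construction script runs LMIUpdate, which pulls shared settings from an optional Control and recomputes the distance, honoring only Y scale.
; It builds a procedural quad with distance-based UVs, colors it through a dynamic material, rotates it toward the target, then adds capped interval labels.
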(event EventGetControlValues
  (|CallParentFunction)
  (Utilities|IsValid (Variables|Default|GetControl)
    (:Is%20Valid
      (Variables|Default|SetShowInterval (Variables|/Game/Lib_LetsMeasureIt/Blueprints/LMI_Control.LMI_Control_C|GetShow%20Interval (Variables|Default|GetControl)))
      (Variables|Default|SetInterval (Variables|/Game/Lib_LetsMeasureIt/Blueprints/LMI_Control.LMI_Control_C|GetInterval (Variables|Default|GetControl)))
      (Variables|Default|SetRulerColor (Variables|/Game/Lib_LetsMeasureIt/Blueprints/LMI_Control.LMI_Control_C|GetRuler%20Color (Variables|Default|GetControl))))))

(event EventLMIUpdate
  (bind _actortarget (Variables|Default|GetActorTarget))
  (Variables|Default|SetUpdate false)
  (CallFunction|GetControlValues)
  ;[1 1 1] Set IntervalCM which is Interval (which is in meters) * 100
  (Variables|Default|SetIntervalCM (Math|Float|Truncate (* (Variables|Default|GetInterval) 1e+02)))
  (Transformation|SetWorldScale3D (Variables|Default|GetTextRender) "1.000000,1.000000,1.000000")
  ;[1 1 1] Handle source and target Actors
  (Utilities|IsValid (Variables|Default|GetActorSource)
    (:Is%20Valid
      (Transformation|SetActorLocation (Transformation|GetActorLocation (Variables|Default|GetActorSource)) false false))
    (:Is%20Not%20Valid
      _))
  (Utilities|IsValid _actortarget
    (:Is%20Valid
      (Variables|Default|SetTargetPoint (- (Transformation|GetActorLocation _actortarget) (Transformation|GetActorLocation))))
    (:Is%20Not%20Valid
      _))
  ;[1 1 1] Ignore scaling on the Actor itself, except Y axis
  (Transformation|SetActorScale3D (Math|Vector|MakeVector 1.0 (.y (Transformation|GetActorScale3D)) 1.0))
  ;[1 1 1] Calculate the length and store it in PointABDistance. Take scaling on the Y axis into account
  (Variables|Default|SetPointABDistance (* (Math|Vector|VectorLength (- (Variables|Default|GetOriginPoint) (Variables|Default|GetTargetPoint))) (.y (Transformation|GetActorScale3D))))
  ;[1 1 1] Set the text of the TextRender to Name and Length
  (Rendering|Components|TextRender|SetText (Variables|Default|GetTextRender) (Utilities|Text|FormatText "{Name}<br>{Length}m" (Utilities|Text|ToText(String) (Utilities|GetDisplayName self)) (Utilities|Text|ToText(Float) (/ (Variables|Default|GetPointABDistance) 1e+02) "HalfToEven" false true 1 324 0 2)))
  (CallFunction|CreateRulerMesh)
  ;[1 1 1] Set the material
  (bind _returnvalue (Rendering|Material|CreateDynamicMaterialInstance "/Game/Lib_LetsMeasureIt/Materials/RulerMAT_Inst.RulerMAT_Inst" "None" "None" :!class /Script/Engine.KismetMaterialLibrary))
  (Rendering|Material|SetVectorParameterValue _returnvalue "Color" (Math|Conversions|ToLinearColor(Color) (Variables|Default|GetRulerColor)) :!class /Script/Engine.MaterialInstanceDynamic)
  (Rendering|Material|SetMaterial (Variables|Default|GetProceduralMesh) 0 _returnvalue)
  ;[1 1 1] Rotate the plane to the TargetPoint
  (Transformation|SetRelativeRotation (Variables|Default|GetProceduralMesh) (Math|Rotator|FindLookatRotation (Variables|Default|GetOriginPoint) (Variables|Default|GetTargetPoint)) false false)
  (CallFunction|CreateIntervalLabels)
  (if (Variables|Default|GetKeepTextCentered)
    ;[1 1 1] Attach component to the mesh and center it on the mesh
    (Transformation|AttachComponentToComponent (Variables|Default|GetTextRender) (Variables|Default|GetProceduralMesh) "None" "KeepRelative" "KeepRelative" "KeepRelative" true)
    (CallFunction|SetupTextTransform (Variables|Default|GetTextRender) (Variables|Default|GetTextColor) self (Math|Transform|MakeTransform (Math|Vector|MakeVector (/ (Variables|Default|GetPointABDistance) 2.0) 0.0 (.z (.location (Variables|Default|GetTextTransform)))) "0,90.000000, 0") (Variables|Default|GetFaceCamera))
    (else
      ;[1 1 1] Attach component to the scene
      (Transformation|AttachComponentToComponent (Variables|Default|GetTextRender) (Variables|Default|GetScene) "None" "KeepRelative" "KeepRelative" "KeepRelative" true)
      ;[1 1 1] Setup text properties
      (CallFunction|SetupTextTransform (Variables|Default|GetTextRender) (Variables|Default|GetTextColor) self (Variables|Default|GetTextTransform) (Variables|Default|GetFaceCamera)))))

(fn ConstructionScript
  (CallFunction|LMIUpdate))

(fn CreateRulerMesh
  (bind _ruleruvs (Variables|Default|GetRulerUVs))
  (bind _pointabdistance (Variables|Default|GetPointABDistance))
  (bind _rulerplanevertices (Variables|Default|GetRulerPlaneVertices))
  (bind _pointabdistance_2 (Variables|Default|GetPointABDistance))
  (bind _returnvalue (/ _pointabdistance 1e+02))
  ;[1 1 1] Fill Vertices array. Indices array is already filled!
  (Utilities|Array|Add _rulerplanevertices "0,0.000000,50.000000")
  (Utilities|Array|Add :TargetArray _rulerplanevertices)
  (Utilities|Array|Add _rulerplanevertices (Math|Vector|MakeVector _pointabdistance_2 0.0 0.0))
  (Utilities|Array|Add _rulerplanevertices (Math|Vector|MakeVector _pointabdistance_2 0.0 5e+01))
  ;[1 1 1] Fill UV's array
  (Utilities|Array|Add _ruleruvs "(X=0.000000,Y=0.000000)")
  (Utilities|Array|Add _ruleruvs (Math|Vector2D|MakeVector2D 0.0 0.5))
  (Utilities|Array|Add _ruleruvs (Math|Vector2D|MakeVector2D _returnvalue 0.5))
  (Utilities|Array|Add _ruleruvs (Math|Vector2D|MakeVector2D _returnvalue 0.0))
  ;[1 1 1] Create the Mesh
  (Class|ProceduralMeshComponent|CreateMeshSectionLinearColor (Variables|Default|GetProceduralMesh) 0 (Variables|Default|GetRulerPlaneVertices) (Variables|Default|GetRulerPlaneIndices) 0 (Variables|Default|GetRulerUVs) 0 0 0 0 0 false))

(fn CreateIntervalLabels
  (for _array_element (Variables|Default|GetTextRenderers)
    (Components|DestroyComponent _array_element))
  (Utilities|Array|Clear (Variables|Default|GetTextRenderers))
  (if (Variables|Default|GetShowInterval)
    (for _index (range 0 (Math|Integer|Clamp(Integer) (Math|Float|Truncate (/ (Variables|Default|GetPointABDistance) (Math|Conversions|ToFloat(Integer) (Variables|Default|GetIntervalCM)))) 0 250))
      ;[1 1 1] Create TextRender and set correct position on the ruler
      (LocalVariables|SetcurrentTextRenderTransform (Math|Transform|MakeTransform (Math|Vector|MakeVector (Math|Conversions|ToFloat(Integer) (* _index (Variables|Default|GetIntervalCM))) 0.0 5e+01) "0,90.000000, 0"))
      (bind _returnvalue (AddComponent|AddTextRenderComponent false))
      (bind _output_get (LocalVariables|SetcurrentTextRender _returnvalue))
      (Utilities|Array|Add (Variables|Default|GetTextRenderers) _output_get)
      ;[1 1 1] Set the text to the current interval
      (Rendering|Components|TextRender|SetText (LocalVariables|GetcurrentTextRender) (Utilities|Text|FormatText "{interval}m" (/ (Math|Conversions|ToFloat(Integer) (* _index (Variables|Default|GetIntervalCM))) 1e+02)))
      ;[1 1 1] Set horizontal alignment to Center
      (Rendering|Components|TextRender|SetHorizontalAlignment (LocalVariables|GetcurrentTextRender) "EHTA_Center")
      ;[1 1 1] Attach the TextRender to the procedural mesh so it follows transformation
      (Transformation|AttachComponentToComponent (LocalVariables|GetcurrentTextRender) (Variables|Default|GetProceduralMesh) "None" "KeepRelative" "KeepRelative" "KeepRelative" true)
      (CallFunction|SetupTextTransform (LocalVariables|GetcurrentTextRender) (Variables|Default|GetTextColor) self (LocalVariables|GetcurrentTextRenderTransform) (Variables|Default|GetFaceCamera)))))