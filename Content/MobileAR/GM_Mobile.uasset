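; GM_Mobile, by name the mobile AR game mode, sets up access to WiTracing wireless signal simulation.
; BeginPlay finds and caches the level's WiTracingAgent.
; A helper fetches and stores the WirelessRX child actor of BP_AI_With_RX.
; An unconnected debug chain would trace transmitters within a fixed radius of that receiver and print each name and RSSI, but never runs.
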(event EventTick
  (params (DeltaSeconds :type Float%20%28single-precision%29)))

(event EventBeginPlay
  (CallFunction|CacheWiTracingAgent))

(fn ConstructionScript)

(fn CacheAIPawnRX
  (bind _returnvalue (Actor|GetActorOfClass "/Game/Demo/Character/BP_AI_With_RX.BP_AI_With_RX_C"))
  (bind _aswireless_rx (Utilities|Casting|CastToWirelessRX (Variables|/Script/Engine.ChildActorComponent|GetChildActor (Variables|/Game/Demo/Character/BP_AI_With_RX.BP_AI_With_RX_C|GetRX _returnvalue))))
  (bind _output_get (Variables|Default|SetWirelessRX _aswireless_rx))
  (return _output_get))

(fn CacheWiTracingAgent
  (bind _returnvalue (Actor|GetActorOfClass "/Script/WiTracingSim.WiTracingAgent"))
  (Variables|Default|SetWTAgent _returnvalue))