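; BP_Door_06 is an automatic sliding double door in the shopping mall.
; Box overlap begin plays a timeline that lerps Door1 and Door2 apart along local Y, and overlap end reverses it.
; A pair of DoOnce nodes, each resetting the other, alternates the sliding sound between opening and closing, playing it at the world origin.
; Overlaps are not filtered by actor or counted.
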(event OnComponentBeginOverlap(Box)
  (params (OverlappedComponent :type Primitive%20Component%20Object%20Reference) (OtherActor :type Actor%20Object%20Reference) (OtherComp :type Primitive%20Component%20Object%20Reference) (OtherBodyIndex :type Integer) (bFromSweep :type Boolean) (SweepResult :type Hit%20Result%20Structure%20%28by%20ref%29))
  (Utilities|FlowControl|Sequence
    (:then_0
      (bind (_direction _newtrack_0 _newtrack_1) (Timeline|Timeline_0 Play)
        (:Update
          (Transformation|SetRelativeLocation (Variables|Default|GetDoor1) (Math|Vector|MakeVector 0.0 (Math|Float|Lerp -226.899689 -123.13781 _newtrack_0) 0.0) false false)
          (Transformation|SetRelativeLocation (Variables|Default|GetDoor2) (Math|Vector|MakeVector 0.0 (Math|Float|Lerp -337.324585 -4.4e+02 _newtrack_1) 0.0) false false))))
    (:then_1
      (Utilities|FlowControl|DoOnce false
        (:Completed
          (Audio|PlaySoundatLocation "/Game/ShoppingMall/Meshes/Door/Sound/Sliding_Door_Cue.Sliding_Door_Cue" "0, 0, 0" "0, 0, 0" 1.0 1.0 0.0 0 0 0)
          (Utilities|FlowControl|DoOnce false) ; enters at Reset
        )))))

(event OnComponentEndOverlap(Box)
  (params (OverlappedComponent :type Primitive%20Component%20Object%20Reference) (OtherActor :type Actor%20Object%20Reference) (OtherComp :type Primitive%20Component%20Object%20Reference) (OtherBodyIndex :type Integer))
  (Utilities|FlowControl|Sequence
    (:then_0
      (bind (_direction _newtrack_0 _newtrack_1) (Timeline|Timeline_0 Reverse)
        (:Update
          (Transformation|SetRelativeLocation (Variables|Default|GetDoor1) (Math|Vector|MakeVector 0.0 (Math|Float|Lerp -226.899689 -123.13781 _newtrack_0) 0.0) false false)
          (Transformation|SetRelativeLocation (Variables|Default|GetDoor2) (Math|Vector|MakeVector 0.0 (Math|Float|Lerp -337.324585 -4.4e+02 _newtrack_1) 0.0) false false))))
    (:then_1
      (Utilities|FlowControl|DoOnce false
        (:Completed
          (Audio|PlaySoundatLocation "/Game/ShoppingMall/Meshes/Door/Sound/Sliding_Door_Cue.Sliding_Door_Cue" "0, 0, 0" "0, 0, 0" 1.0 1.0 0.0 0 0 0)
          (Utilities|FlowControl|DoOnce false) ; enters at Reset
        )))))

(fn ConstructionScript)