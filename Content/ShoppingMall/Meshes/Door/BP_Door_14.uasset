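; BP_Door_14 is an interactive shopping mall door that slides along its relative Z axis.
; A box overlap enables player input, and Oninteract flip-flops a timeline between play and reverse to move the door.
; Two cross-resetting DoOnce nodes gate the rising-gate sound, which plays at world origin.
; Any actor beginning overlap with the door actor stops the timeline.
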(event OnComponentBeginOverlap(Box)
  (params (OverlappedComponent :type Primitive%20Component%20Object%20Reference) (OtherActor :type Actor%20Object%20Reference) (OtherComp :type Primitive%20Component%20Object%20Reference) (OtherBodyIndex :type Integer) (bFromSweep :type Boolean) (SweepResult :type Hit%20Result%20Structure%20%28by%20ref%29))
  (Input|EnableInput (Game|GetPlayerController 0)))

(event OnComponentEndOverlap(Box)
  (params (OverlappedComponent :type Primitive%20Component%20Object%20Reference) (OtherActor :type Actor%20Object%20Reference) (OtherComp :type Primitive%20Component%20Object%20Reference) (OtherBodyIndex :type Integer))
  (Input|DisableInput (Game|GetPlayerController 0)))

(event Collision|EventActorBeginOverlap
  (params (OtherActor :type Actor%20Object%20Reference))
  (bind _door (Timeline|Timeline_1 Stop)
    (:Update
      (Transformation|SetRelativeLocation (Variables|Default|GetDoor) (Math|Vector|MakeVector 0.0 0.0 _door) false false))))

(event EventOninteract
  (Utilities|FlowControl|FlipFlop
    (:A
      (Utilities|FlowControl|Sequence
        (:then_0
          (Utilities|FlowControl|DoOnce false :!label _label
            (:Completed
              (Audio|PlaySoundatLocation "/Game/ShoppingMall/Meshes/Door/Sound/Rising_Gates_Cue_01.Rising_Gates_Cue_01" "0, 0, 0" "0, 0, 0" 1.0 1.0 0.0 0 0 0)
              (goto _label_2 Reset))))
        (:then_1
          (bind _door (Timeline|Timeline_1 Play)
            (:Update
              (Transformation|SetRelativeLocation (Variables|Default|GetDoor) (Math|Vector|MakeVector 0.0 0.0 _door) false false))))))
    (:B
      (Utilities|FlowControl|Sequence
        (:then_0
          (Timeline|Timeline_1 Reverse))
        (:then_1
          (Utilities|FlowControl|DoOnce false :!label _label_2
            (:Completed
              (Audio|PlaySoundatLocation "/Game/ShoppingMall/Meshes/Door/Sound/Rising_Gates_Cue_01.Rising_Gates_Cue_01" "0, 0, 0" "0, 0, 0" 1.0 1.0 0.0 0 0 0)
              (goto _label Reset))))))))

(fn ConstructionScript)