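; Three-floor shopping mall elevator with animated inner doors, floor buttons, a stop button and sound cues.
; Floor events pass a single-press guard, close the doors, then reopen them if already there or play a timeline forward or backward.
; The timeline moves the cabin along a spline's Z until the target floor's point.
; Landing doors are separate BP_Elevator01_Doors1 actors, picked by floor index from GetAllActorsOfClass.
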(event Custom|OpenInnerDoor
  (bind _innerdoor_r_ (Variables|Default|GetInnerDoor%28R%29))
  (bind _relativelocation (Variables|/Script/Engine.SceneComponent|GetRelativeLocation _innerdoor_r_))
  ;[1 1 1] Opening elevator doors (Inner Doors)
  (Variables|Default|SetRightInnerDoor (.y _relativelocation))
  (bind _newtrack_0 (Timeline|InnerDoorOpen PlayFromStart)
    (:Update
      (bind _result (Math|Float|NegateFloat _newtrack_0)
        (:%20%20
          (Transformation|SetRelativeLocation _innerdoor_r_ (Math|Vector|MakeVector (.x _relativelocation) (- (Variables|Default|GetRightInnerDoor) _result) (.z _relativelocation)) false false)
          (Transformation|SetRelativeLocation (Variables|Default|GetInnerDoor%28L%29) (Math|Vector|MakeVector (.x _relativelocation) _newtrack_0 (.z _relativelocation)) false false))))))

(event Custom|CloseInnerDoor
  (bind _innerdoor_r_ (Variables|Default|GetInnerDoor%28R%29))
  (bind _relativelocation (Variables|/Script/Engine.SceneComponent|GetRelativeLocation _innerdoor_r_))
  ;[1 1 1] Opening elevator doors (Inner Doors)
  (bind _newtrack_0 (Timeline|InnerDoorOpen ReverseFromEnd)
    (:Update
      (bind _result (Math|Float|NegateFloat _newtrack_0)
        (:%20%20
          (Transformation|SetRelativeLocation _innerdoor_r_ (Math|Vector|MakeVector (.x _relativelocation) (- (Variables|Default|GetRightInnerDoor) _result) (.z _relativelocation)) false false)
          (Transformation|SetRelativeLocation (Variables|Default|GetInnerDoor%28L%29) (Math|Vector|MakeVector (.x _relativelocation) _newtrack_0 (.z _relativelocation)) false false))))))

(event Custom|Stop_Elevator
  (bind _spline (Variables|Default|GetSpline))
  (bind _spline_2 (Variables|Default|GetSpline))
  (bind _button04 (Variables|Default|Getbutton04))
  (bind _relativescale3d (Variables|/Script/Engine.SceneComponent|GetRelativeScale3D _button04))
  ;[1 1 1] Elevator Stop Button
  (Audio|Components|Audio|Play (Variables|Default|GetPressingTheButton_Cue) 0.0)
  (bind _newtrack_0 (Timeline|Press_Stop_Elevator PlayFromStart)
    (:Update
      (Transformation|SetRelativeScale3D _button04 (Math|Vector|MakeVector _newtrack_0 (.y _relativescale3d) (.z _relativescale3d)))
      (Variables|Default|SetIsTheElevator_Call_ButtonPressed false)
      (Audio|Components|Audio|Stop (Variables|Default|GetElevatorMovement_Cue))
      (bind (_direction _newtrack_0_2) (Timeline|Timeline_0 Stop)
        (:Update
          (switch Utilities|FlowControl|Switch|SwitchonETimelineDirection _direction
            (:Forward
              ;[1 1 1] The elevator rises
              (if (< (.z (Spline|GetLocationatTime _spline_2 _newtrack_0_2 "Local" false)) (.z (Spline|GetLocationatSplinePoint _spline_2 (Variables|Default|GetWhich_Floor_do_You_Need) "Local")))
                (Transformation|SetRelativeLocation (Variables|Default|GetElevator) (Math|Vector|MakeVector 0.0 0.0 (.z (Spline|GetLocationatTime _spline_2 _newtrack_0_2 "Local" false))) false false)
                (else
                  (Variables|Default|SetWhere_Is_TheElevatorNow (Variables|Default|GetWhich_Floor_do_You_Need))
                  (bind _outactors (Actor|GetAllActorsOfClass "/Game/ShoppingMall/Meshes/Elevator/BP_Elevator01_Doors1.BP_Elevator01_Doors1_C" :!label _label))
                  (Default|OpenDoors (Utilities|Array|Get(acopy) _outactors (Variables|Default|GetWhich_Floor_do_You_Need)))
                  (CallFunction|OpenInnerDoor)
                  (Variables|Default|SetDoors_are_closed_or_open false)
                  (Variables|Default|SetIsTheElevator_Call_ButtonPressed false)
                  (Audio|Components|Audio|Stop (Variables|Default|GetElevatorMovement_Cue))
                  (Audio|Components|Audio|Play (Variables|Default|GetOpenDoor_Cue1) -1.0)
                  (Timeline|Timeline_0 Stop))))
            (:Backward
              ;[1 1 1] The elevator descends
              (if (> (.z (Spline|GetLocationatTime _spline _newtrack_0_2 "Local" false)) (.z (Spline|GetLocationatSplinePoint _spline (Variables|Default|GetWhich_Floor_do_You_Need) "Local")))
                (Transformation|SetRelativeLocation (Variables|Default|GetElevator) (Math|Vector|MakeVector 0.0 0.0 (.z (Spline|GetLocationatTime _spline _newtrack_0_2 "Local" false))) false false)
                (else
                  (Variables|Default|SetWhere_Is_TheElevatorNow (Variables|Default|GetWhich_Floor_do_You_Need))
                  (goto _label))))))))))

(event Custom|1_Floor
  (bind _spline (Variables|Default|GetSpline))
  (bind _spline_2 (Variables|Default|GetSpline))
  (bind _button01 (Variables|Default|Getbutton01))
  (bind _relativescale3d (Variables|/Script/Engine.SceneComponent|GetRelativeScale3D _button01))
  ;[1 1 1] The elevator buttons are associated with the player's blueprint.
  (Audio|Components|Audio|Play (Variables|Default|GetElevatorMovement_Cue) 0.0)
  (Utilities|NewMacro2
    (:PerformTheAction
      (CallFunction|DoorFunction)
      ;[1 1 1] Elevator Floor Buttons Animation
      (bind _newtrack_0 (Timeline|Pressing%20the%20button%2001%20%281st%20floor%29 PlayFromStart)
        (:Update
          (Transformation|SetRelativeScale3D _button01 (Math|Vector|MakeVector _newtrack_0 (.y _relativescale3d) (.z _relativescale3d)))
          (Utilities|FlowControl|Delay 1.5)
          (bind _output_get (Variables|Default|SetWhich_Floor_do_You_Need 0))
          (Utilities|NewMacro1
            (:GO
              (Math|Integer|CompareInt _output_get (Variables|Default|GetWhere_Is_TheElevatorNow)
                (:>
                  (bind (_direction _newtrack_0_2) (Timeline|Timeline_0 Play)
                    (:Update
                      (switch Utilities|FlowControl|Switch|SwitchonETimelineDirection _direction
                        (:Forward
                          ;[1 1 1] The elevator rises
                          (if (< (.z (Spline|GetLocationatTime _spline_2 _newtrack_0_2 "Local" false)) (.z (Spline|GetLocationatSplinePoint _spline_2 (Variables|Default|GetWhich_Floor_do_You_Need) "Local")))
                            (Transformation|SetRelativeLocation (Variables|Default|GetElevator) (Math|Vector|MakeVector 0.0 0.0 (.z (Spline|GetLocationatTime _spline_2 _newtrack_0_2 "Local" false))) false false)
                            (else
                              (Variables|Default|SetWhere_Is_TheElevatorNow (Variables|Default|GetWhich_Floor_do_You_Need))
                              (bind _outactors (Actor|GetAllActorsOfClass "/Game/ShoppingMall/Meshes/Elevator/BP_Elevator01_Doors1.BP_Elevator01_Doors1_C" :!label _label))
                              (Default|OpenDoors (Utilities|Array|Get(acopy) _outactors (Variables|Default|GetWhich_Floor_do_You_Need)))
                              (CallFunction|OpenInnerDoor)
                              (Variables|Default|SetDoors_are_closed_or_open false)
                              (Variables|Default|SetIsTheElevator_Call_ButtonPressed false)
                              (Audio|Components|Audio|Stop (Variables|Default|GetElevatorMovement_Cue))
                              (Audio|Components|Audio|Play (Variables|Default|GetOpenDoor_Cue1) -1.0)
                              (Timeline|Timeline_0 Stop))))
                        (:Backward
                          ;[1 1 1] The elevator descends
                          (if (> (.z (Spline|GetLocationatTime _spline _newtrack_0_2 "Local" false)) (.z (Spline|GetLocationatSplinePoint _spline (Variables|Default|GetWhich_Floor_do_You_Need) "Local")))
                            (Transformation|SetRelativeLocation (Variables|Default|GetElevator) (Math|Vector|MakeVector 0.0 0.0 (.z (Spline|GetLocationatTime _spline _newtrack_0_2 "Local" false))) false false)
                            (else
                              (Variables|Default|SetWhere_Is_TheElevatorNow (Variables|Default|GetWhich_Floor_do_You_Need))
                              (goto _label))))))))
                (:<
                  (Timeline|Timeline_0 Reverse))))))))))

(event Custom|2_Floor
  (bind _spline (Variables|Default|GetSpline))
  (bind _spline_2 (Variables|Default|GetSpline))
  (bind _button02 (Variables|Default|Getbutton02))
  (bind _relativescale3d (Variables|/Script/Engine.SceneComponent|GetRelativeScale3D _button02))
  ;[1 1 1] The elevator buttons are associated with the player's blueprint.
  (Audio|Components|Audio|Play (Variables|Default|GetElevatorMovement_Cue) 0.0)
  (Utilities|NewMacro2
    (:PerformTheAction
      (CallFunction|DoorFunction)
      ;[1 1 1] Elevator Floor Buttons Animation
      (bind _newtrack_0 (Timeline|Pressing%20the%20button%20%282st%20floor%29 PlayFromStart)
        (:Update
          (Transformation|SetRelativeScale3D _button02 (Math|Vector|MakeVector _newtrack_0 (.y _relativescale3d) (.z _relativescale3d)))
          (Utilities|FlowControl|Delay 1.5)
          (bind _output_get (Variables|Default|SetWhich_Floor_do_You_Need 1))
          (Utilities|NewMacro1
            (:GO
              (Math|Integer|CompareInt _output_get (Variables|Default|GetWhere_Is_TheElevatorNow)
                (:>
                  (bind (_direction _newtrack_0_2) (Timeline|Timeline_0 Play)
                    (:Update
                      (switch Utilities|FlowControl|Switch|SwitchonETimelineDirection _direction
                        (:Forward
                          ;[1 1 1] The elevator rises
                          (if (< (.z (Spline|GetLocationatTime _spline_2 _newtrack_0_2 "Local" false)) (.z (Spline|GetLocationatSplinePoint _spline_2 (Variables|Default|GetWhich_Floor_do_You_Need) "Local")))
                            (Transformation|SetRelativeLocation (Variables|Default|GetElevator) (Math|Vector|MakeVector 0.0 0.0 (.z (Spline|GetLocationatTime _spline_2 _newtrack_0_2 "Local" false))) false false)
                            (else
                              (Variables|Default|SetWhere_Is_TheElevatorNow (Variables|Default|GetWhich_Floor_do_You_Need))
                              (bind _outactors (Actor|GetAllActorsOfClass "/Game/ShoppingMall/Meshes/Elevator/BP_Elevator01_Doors1.BP_Elevator01_Doors1_C" :!label _label))
                              (Default|OpenDoors (Utilities|Array|Get(acopy) _outactors (Variables|Default|GetWhich_Floor_do_You_Need)))
                              (CallFunction|OpenInnerDoor)
                              (Variables|Default|SetDoors_are_closed_or_open false)
                              (Variables|Default|SetIsTheElevator_Call_ButtonPressed false)
                              (Audio|Components|Audio|Stop (Variables|Default|GetElevatorMovement_Cue))
                              (Audio|Components|Audio|Play (Variables|Default|GetOpenDoor_Cue1) -1.0)
                              (Timeline|Timeline_0 Stop))))
                        (:Backward
                          ;[1 1 1] The elevator descends
                          (if (> (.z (Spline|GetLocationatTime _spline _newtrack_0_2 "Local" false)) (.z (Spline|GetLocationatSplinePoint _spline (Variables|Default|GetWhich_Floor_do_You_Need) "Local")))
                            (Transformation|SetRelativeLocation (Variables|Default|GetElevator) (Math|Vector|MakeVector 0.0 0.0 (.z (Spline|GetLocationatTime _spline _newtrack_0_2 "Local" false))) false false)
                            (else
                              (Variables|Default|SetWhere_Is_TheElevatorNow (Variables|Default|GetWhich_Floor_do_You_Need))
                              (goto _label))))))))
                (:<
                  (Timeline|Timeline_0 Reverse))))))))))

(event Custom|3_Floor
  (bind _spline (Variables|Default|GetSpline))
  (bind _spline_2 (Variables|Default|GetSpline))
  (bind _button03 (Variables|Default|Getbutton03))
  (bind _relativescale3d (Variables|/Script/Engine.SceneComponent|GetRelativeScale3D _button03))
  ;[1 1 1] The elevator buttons are associated with the player's blueprint.
  (Audio|Components|Audio|Play (Variables|Default|GetElevatorMovement_Cue) 0.0)
  (Utilities|NewMacro2
    (:PerformTheAction
      (CallFunction|DoorFunction)
      ;[1 1 1] Elevator Floor Buttons Animation
      (bind _newtrack_0 (Timeline|Pressing%20the%20button%2003%20%20%283st%20floor%29 PlayFromStart)
        (:Update
          (Transformation|SetRelativeScale3D _button03 (Math|Vector|MakeVector _newtrack_0 (.y _relativescale3d) (.z _relativescale3d)))
          (Utilities|FlowControl|Delay 1.5)
          (bind _output_get (Variables|Default|SetWhich_Floor_do_You_Need 2))
          (Utilities|NewMacro1
            (:GO
              (Math|Integer|CompareInt _output_get (Variables|Default|GetWhere_Is_TheElevatorNow)
                (:>
                  (bind (_direction _newtrack_0_2) (Timeline|Timeline_0 Play)
                    (:Update
                      (switch Utilities|FlowControl|Switch|SwitchonETimelineDirection _direction
                        (:Forward
                          ;[1 1 1] The elevator rises
                          (if (< (.z (Spline|GetLocationatTime _spline_2 _newtrack_0_2 "Local" false)) (.z (Spline|GetLocationatSplinePoint _spline_2 (Variables|Default|GetWhich_Floor_do_You_Need) "Local")))
                            (Transformation|SetRelativeLocation (Variables|Default|GetElevator) (Math|Vector|MakeVector 0.0 0.0 (.z (Spline|GetLocationatTime _spline_2 _newtrack_0_2 "Local" false))) false false)
                            (else
                              (Variables|Default|SetWhere_Is_TheElevatorNow (Variables|Default|GetWhich_Floor_do_You_Need))
                              (bind _outactors (Actor|GetAllActorsOfClass "/Game/ShoppingMall/Meshes/Elevator/BP_Elevator01_Doors1.BP_Elevator01_Doors1_C" :!label _label))
                              (Default|OpenDoors (Utilities|Array|Get(acopy) _outactors (Variables|Default|GetWhich_Floor_do_You_Need)))
                              (CallFunction|OpenInnerDoor)
                              (Variables|Default|SetDoors_are_closed_or_open false)
                              (Variables|Default|SetIsTheElevator_Call_ButtonPressed false)
                              (Audio|Components|Audio|Stop (Variables|Default|GetElevatorMovement_Cue))
                              (Audio|Components|Audio|Play (Variables|Default|GetOpenDoor_Cue1) -1.0)
                              (Timeline|Timeline_0 Stop))))
                        (:Backward
                          ;[1 1 1] The elevator descends
                          (if (> (.z (Spline|GetLocationatTime _spline _newtrack_0_2 "Local" false)) (.z (Spline|GetLocationatSplinePoint _spline (Variables|Default|GetWhich_Floor_do_You_Need) "Local")))
                            (Transformation|SetRelativeLocation (Variables|Default|GetElevator) (Math|Vector|MakeVector 0.0 0.0 (.z (Spline|GetLocationatTime _spline _newtrack_0_2 "Local" false))) false false)
                            (else
                              (Variables|Default|SetWhere_Is_TheElevatorNow (Variables|Default|GetWhich_Floor_do_You_Need))
                              (goto _label))))))))
                (:<
                  (Timeline|Timeline_0 Reverse))))))))))

(fn ConstructionScript)

(fn DoorFunction
  ;[1 1 1] Closing internal and external elevator doors
  (if (Variables|Default|GetFirstDoor)
    (Variables|Default|SetFirstDoor false)
    (elif (Variables|Default|GetDoors_are_closed_or_open)
      _
      (else
        (bind _outactors (Actor|GetAllActorsOfClass "/Game/ShoppingMall/Meshes/Elevator/BP_Elevator01_Doors1.BP_Elevator01_Doors1_C"))
        (Default|CloseDoors (Utilities|Array|Get(acopy) _outactors (Variables|Default|GetWhere_Is_TheElevatorNow)))
        (CallFunction|CloseInnerDoor)
        (Variables|Default|SetDoors_are_closed_or_open true)
        (Audio|Components|Audio|Play (Variables|Default|GetOpenDoor_Cue1) -1.0))))
  (return))