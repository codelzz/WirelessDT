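; Elevator door Blueprint for the shopping mall that slides two lift door meshes open and closed.
; A DoorOpen timeline drives both doors along relative Y, offsetting the left from its position stored on opening and setting the right directly from the track value.
; Closing reverses the same timeline from its end.
; Open and close are custom events with no trigger inside this Blueprint, and overlap and tick are disabled.
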(event Custom|OpenDoors%282%29
  (bind _lift_door_l_ (Variables|Default|GetLift_door%28L%29))
  (Variables|Default|SetLeftDoor (.y (Variables|/Script/Engine.SceneComponent|GetRelativeLocation _lift_door_l_)))
  (bind _newtrack_0 (Timeline|DoorOpen Play)
    (:Update
      (bind _result (Math|Float|NegateFloat _newtrack_0)
        (:%20%20
          (Transformation|SetRelativeLocation _lift_door_l_ (Math|Vector|MakeVector 0.0 (- (Variables|Default|GetLeftDoor) _result) 0.0) false false)
          (Transformation|SetRelativeLocation (Variables|Default|GetLift_door%28R%29) (Math|Vector|MakeVector 0.0 _newtrack_0 0.0) false false))))))

(event Custom|CloseDoors%282%29
  (bind _newtrack_0 (Timeline|DoorOpen ReverseFromEnd)
    (:Update
      (bind _result (Math|Float|NegateFloat _newtrack_0)
        (:%20%20
          (Transformation|SetRelativeLocation (Variables|Default|GetLift_door%28L%29) (Math|Vector|MakeVector 0.0 (- (Variables|Default|GetLeftDoor) _result) 0.0) false false)
          (Transformation|SetRelativeLocation (Variables|Default|GetLift_door%28R%29) (Math|Vector|MakeVector 0.0 _newtrack_0 0.0) false false))))))

(event Collision|EventActorBeginOverlap
  (params (OtherActor :type Actor%20Object%20Reference)))

(event EventTick
  (params (DeltaSeconds :type Float%20%28single-precision%29)))

(fn ConstructionScript)